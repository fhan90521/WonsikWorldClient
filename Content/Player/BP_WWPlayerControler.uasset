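; Player controller for a networked game that handles click-to-move, chat, near/far camera views, obstacle spawning and field map loading.
; SCBP events spawn the local and other players as AI pawns, storing others by player ID for nicknamed chat.
; Right-click traces under the cursor, stops current movement and passes the destination to MoveMyCharacterCS.
; Outgoing chat shows locally through ACUIManager, then goes to SendChatMessageCS.
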(event `self.ReceiveBeginPlay`
  (set `self.bShowMouseCursor` true))

(event `self.ShowCurMapID_BP`
  (params (mapID :type Integer))
  (`/Game/UI/WB_PlayerUI.ShowCurrentMapID` (`/Game/UI/AC_UIManager.UIRef` (`self.AC_UIManager`)) mapID))

(event `self.CreateObstacle_BP`
  (params (x :type "Float (single-precision)") (y :type "Float (single-precision)"))
  (`|SpawnActorFromClass` "/Game/Field/obstacle.obstacle_C" (`KismetMathLibrary.Conv_VectorToTransform` (`KismetMathLibrary.MakeVector` x y)) "Undefined" "MultiplyWithRoot" null null))

(event `self.ChangeMapSC_BP`
  (params (afterMapID :type Integer))
  (`GameplayStatics.OpenLevelBySoftObjectPtr` "/Game/Field/WWFieldMap.WWFieldMap"))

(event `self.CreateOtherCharacterSC_BP`
  (params (playerID :type Integer64) (nickName :type String) (dirVec :type "Vector Structure (by ref)") (location :type "Vector Structure (by ref)"))
  (if (`BlueprintMapLibrary.Map_Contains` (`self.OtherCharacters`) playerID)
    (`KismetSystemLibrary.PrintString` "Already other character exist error" true true (struct :`R` 1.0 :`G` 0.15429 :`B` 0.124442 :`A` 1.0))
    (else
      (bind _returnvalue (`AIBlueprintHelperLibrary.SpawnAIFromClass` "/Game/Player/BP_WWOtherCharacter.BP_WWOtherCharacter_C" null location (`KismetMathLibrary.Conv_VectorToRotator` dirVec) true null))
      (bind _asbp_wwother_character (cast `/Game/Player/BP_WWOtherCharacter` _returnvalue)
        (:`then`
          (`BlueprintMapLibrary.Map_Add` (`self.OtherCharacters`) playerID _asbp_wwother_character)
          (`/Game/Player/BP_WWOtherCharacter.SetOtherNickName` _asbp_wwother_character nickName))
        (:`CastFailed`
          (`KismetSystemLibrary.PrintString` "Spawn other Character Fail"))))))

(event `self.CreateMyCharacterSC_BP`
  (params (dirVec :type "Vector Structure (by ref)") (location :type "Vector Structure (by ref)"))
  (bind _returnvalue (`AIBlueprintHelperLibrary.SpawnAIFromClass` "/Game/Player/BP_WWPlayerCharacter.BP_WWPlayerCharacter_C" null location (`KismetMathLibrary.Conv_VectorToRotator` dirVec) true null))
  (bind _asbp_wwplayer_character (cast `/Game/Player/BP_WWPlayerCharacter` _returnvalue)
    (:`then`
      (`/Game/Player/BP_WWPlayerCharacter.SetMyNick Name` _asbp_wwplayer_character (`self.MyFNickName`))
      (bind _output_get (set `self.MyCharacter` _asbp_wwplayer_character))
      (`self.SetViewTargetWithBlend` _output_get))
    (:`CastFailed`
      (`KismetSystemLibrary.PrintString` "Spawn My Character FAIL"))))

(event `Key|RightMouseButton`
  (params (Key :type "Key Structure"))
  (bind (_worldlocation _worlddirection) (`self.DeprojectMousePositionToWorld` (`GameplayStatics.GetPlayerController` 0)))
  (:`Pressed`
    (if (`KismetSystemLibrary.IsValid` (`self.MyCharacter`))
      (bind (_outhit _returnvalue) (`KismetSystemLibrary.LineTraceSingle` _worldlocation (+ _worldlocation (* _worlddirection 10000.0)) "TraceTypeQuery1"))
      (if _returnvalue
        (`self.StopMovement` (`AIBlueprintHelperLibrary.GetAIController` (`self.MyCharacter`)))
        (`self.MoveMyCharacterCS` (`.Location` (`GameplayStatics.BreakHitResult` _outhit)))))))

(event `self.SendChatMessageSC_BP`
  (params (playerID :type Integer64) (chatMessage :type String))
  (bind (_value _returnvalue) (`BlueprintMapLibrary.Map_Find` (`self.OtherCharacters`) playerID))
  (if _returnvalue
    (bind _asbp_wwother_character (cast `/Game/Player/BP_WWOtherCharacter` _value))
    (`/Game/UI/AC_UIManager.AddChatMessageOnChatBox` (`self.AC_UIManager`) (`/Game/Player/BP_WWOtherCharacter.OtherNickName` _asbp_wwother_character) chatMessage)
    (else
      (`KismetSystemLibrary.PrintString` "none exist player chat recv error"))))

(event `Key|One`
  (params (Key :type "Key Structure"))
  (:`Pressed`
    (bind _asbp_wwplayer_character (cast `/Game/Player/BP_WWPlayerCharacter` (`self.MyCharacter`)))
    (`/Game/Player/BP_WWPlayerCharacter.ChangeToNearView` _asbp_wwplayer_character)))

(event `Key|Two`
  (params (Key :type "Key Structure"))
  (:`Pressed`
    (bind _asbp_wwplayer_character (cast `/Game/Player/BP_WWPlayerCharacter` (`self.MyCharacter`)))
    (`/Game/Player/BP_WWPlayerCharacter.ChangeToFarView ` _asbp_wwplayer_character)))

(fn `SendChatMessage`
  (params (Message :type String))
  (`/Game/UI/AC_UIManager.AddChatMessageOnChatBox` (`self.AC_UIManager`) (`self.MyFNickName`) Message)
  (`self.SendChatMessageCS` Message))

(fn `UserConstructionScript`)