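; BP_WWOtherCharacter is a character Blueprint that, by its naming, represents another player and carries a nickname tag.
; On BeginPlay it sets the capsule, mesh and NickNameTag component to ignore the Camera collision channel, so they do not block camera traces.
; SetOtherNickName stores the given name and forwards it to the WB_NickNameTag widget held by that component.
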(event `self.ReceiveBeginPlay`
  (`PrimitiveComponent.SetCollisionResponseToChannel` (`self.CapsuleComponent`) "ECC_Camera" "ECR_Ignore")
  (`PrimitiveComponent.SetCollisionResponseToChannel` (`self.Mesh`) "ECC_Camera" "ECR_Ignore")
  (`PrimitiveComponent.SetCollisionResponseToChannel` (`self.NickNameTag`) "ECC_Camera" "ECR_Ignore"))

(fn `SetOtherNickName`
  (params (NickName :type String))
  (bind _output_get (set `self.OtherNickName` NickName))
  (bind _aswb_nick_name_tag (cast `/Game/Player/WB_NickNameTag` (`WidgetComponent.GetWidget` (`self.NickNameTag`))))
  (`/Game/Player/WB_NickNameTag.SetOtherNickName` _aswb_nick_name_tag _output_get))

(fn `UserConstructionScript`)